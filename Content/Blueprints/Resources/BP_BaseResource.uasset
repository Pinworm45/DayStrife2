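; BP_BaseResource is a resource actor with a type, such as Wood or Stone, and a count of units held.
; The Construction Script derives that count from the actor's rounded, clamped X scale, doubling it for Wood and for Stone above the minimum size.
; SubtractResource removes one unit per call and destroys the actor once none remain.
; The event graph holds no active logic.
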(event EventBeginPlay)

(event Collision|EventActorBeginOverlap
  (params (OtherActor :type Actor%20Object%20Reference)))

(event EventTick
  (params (DeltaSeconds :type Float%20%28single-precision%29)))

(fn ConstructionScript
  (bind _returnvalue (Transformation|GetActorScale3D))
  (bind _x (Math|Vector|BreakVector _returnvalue))
  (bind _returnvalue_2 (Math|Float|Round _x))
  (bind _returnvalue_3 (Math|Integer|Clamp(Integer) _returnvalue_2 1 10))
  (switch Utilities|FlowControl|Switch|SwitchonEnumResourceTypes (Variables|Default|GetResourceType)
    (:NewEnumerator0
      (Variables|Default|SetResourcesHeld (* (Math|Integer|Clamp(Integer) (Math|Float|Round (.X (Math|Vector|BreakVector (Transformation|GetActorScale3D)))) 1 10) 2)))
    (:NewEnumerator1
      (if (> _returnvalue_3 1)
        (Variables|Default|SetResourcesHeld (* _returnvalue_3 2))
        (else
          (Variables|Default|SetResourcesHeld _returnvalue_3))))))

(fn SubtractResource
  (bind _output_get (Variables|Default|SetResourcesHeld (- (Variables|Default|GetResourcesHeld) 1)))
  (if (<= _output_get 0)
    (Actor|DestroyActor)))