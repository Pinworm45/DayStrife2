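; Trigger sphere actor that lets its owning AI harvest a wood or stone resource when that AI overlaps it.
; The owner loops a jump animation during a short delay, then returns to walking.
; The sphere removes the owner's nearest instance from the matching tree or rock spawner's instanced static meshes and credits the resource.
; It then clears the owner's task, updates its weight, makes it find new work and destroys itself.
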(event OnComponentBeginOverlap(Sphere)
  (params (OverlappedComponent :type Primitive%20Component%20Object%20Reference) (OtherActor :type Actor%20Object%20Reference) (OtherComp :type Primitive%20Component%20Object%20Reference) (OtherBodyIndex :type Integer) (bFromSweep :type Boolean) (SweepResult :type Hit%20Result%20Structure%20%28by%20ref%29))
  (bind _owningactor (Variables|Default|GetOwningActor))
  (bind _resourcespawnerindex (Variables|/Game/Blueprints/Pawns/TopDownCharacter.TopDownCharacter_C|GetResourceSpawnerIndex _owningactor))
  (bind _nearestinstanceindex (Variables|/Game/Blueprints/Pawns/TopDownCharacter.TopDownCharacter_C|GetNearestInstanceIndex _owningactor))
  (bind _instancetypeindex (Variables|/Game/Blueprints/Pawns/TopDownCharacter.TopDownCharacter_C|GetInstanceTypeIndex _owningactor))
  (bind _arrayoftreespawners (Variables|/Game/Blueprints/Pawns/TopDownCharacter.TopDownCharacter_C|GetArrayOfTreeSpawners _owningactor))
  (bind _mesh (Variables|/Script/Engine.Character|GetMesh _owningactor))
  (bind _arrayofrockspawners (Variables|/Game/Blueprints/Pawns/TopDownCharacter.TopDownCharacter_C|GetArrayOfRockSpawners _owningactor))
  (bind _item (Utilities|Array|Get(acopy) _arrayofrockspawners _resourcespawnerindex))
  (bind _item_2 (Utilities|Array|Get(acopy) _arrayoftreespawners _resourcespawnerindex))
  (if (== OtherActor _owningactor)
    (Components|Animation|PlayAnimation _mesh "/Game/Mannequin/Animations/ThirdPersonJump_Loop.ThirdPersonJump_Loop" true)
    (Utilities|FlowControl|Delay 1.0)
    (Components|Animation|PlayAnimation _mesh "/Game/Mannequin/Animations/ThirdPersonWalk.ThirdPersonWalk" true)
    (switch Utilities|FlowControl|Switch|SwitchonEnumResourceTypes (Variables|Default|GetResourceType)
      (:NewEnumerator0
        (switch int _instancetypeindex
          (:0
            (Class|InstancedStaticMeshComponent|RemoveInstance (Variables|/Game/Blueprints/Resources/BaseTreeSpawner.BaseTreeSpawner_C|GetInstancedStaticMesh _item_2) _nearestinstanceindex))
          (:1
            (Class|InstancedStaticMeshComponent|RemoveInstance (Variables|/Game/Blueprints/Resources/BaseTreeSpawner.BaseTreeSpawner_C|GetInstancedStaticMesh1 _item_2) _nearestinstanceindex))
          (:2
            (Class|InstancedStaticMeshComponent|RemoveInstance (Variables|/Game/Blueprints/Resources/BaseTreeSpawner.BaseTreeSpawner_C|GetInstancedStaticMesh2 _item_2) _nearestinstanceindex)))
        (Default|AddResource _owningactor "NewEnumerator0" 3))
      (:NewEnumerator1
        (switch int _instancetypeindex
          (:0
            (Class|InstancedStaticMeshComponent|RemoveInstance (Variables|/Game/Blueprints/Resources/BaseRockSpawner.BaseRockSpawner_C|GetInstancedStaticMesh _item) _nearestinstanceindex))
          (:1
            (Class|InstancedStaticMeshComponent|RemoveInstance (Variables|/Game/Blueprints/Resources/BaseRockSpawner.BaseRockSpawner_C|GetInstancedStaticMesh1 _item) _nearestinstanceindex))
          (:2
            (Class|InstancedStaticMeshComponent|RemoveInstance (Variables|/Game/Blueprints/Resources/BaseRockSpawner.BaseRockSpawner_C|GetInstancedStaticMesh2 _item) _nearestinstanceindex)))
        (Default|AddResource _owningactor "NewEnumerator1" 3)))
    (Variables|/Game/Blueprints/Pawns/TopDownCharacter.TopDownCharacter_C|SetHasTask _owningactor false)
    (Default|UpdateWeight _owningactor)
    (Default|FindTasktoDo (Variables|Default|GetOwningActor))
    (Actor|DestroyActor)))

(event EventBeginPlay)

(fn ConstructionScript)