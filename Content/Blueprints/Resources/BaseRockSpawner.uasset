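; Base rock spawner that procedurally scatters instanced meshes over landscape around the actor, entirely in the Construction Script.
; Each iteration runs a debug-drawn visibility trace toward lower Z using random XY offsets within Distance.
; Hits on actors tagged "landscape" add an instance to one of three Instanced Static Mesh components, with random yaw and uniform scale.
; The Seed stream drives all randomness, and TotalTrees sets the attempt count despite the rock naming.
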(event EventBeginPlay)

(event Collision|EventActorBeginOverlap
  (params (OtherActor :type Actor%20Object%20Reference)))

(event EventTick
  (params (DeltaSeconds :type Float%20%28single-precision%29)))

(fn ConstructionScript
  (bind _returnvalue (Transformation|GetActorLocation))
  (bind _distance (Variables|Default|GetDistance))
  (bind _seed (Variables|Default|GetSeed))
  (bind _seed_2 (Variables|Default|GetSeed))
  (bind _distance_2 (Variables|Default|GetDistance))
  (bind (_x _y _z) (Math|Vector|BreakVector _returnvalue))
  (bind _returnvalue_2 (* _distance_2 -1.0))
  (bind _returnvalue_3 (* _distance -1.0))
  (bind _returnvalue_4 (Math|Random|RandomFloatinRangefromStream _returnvalue_2 _distance_2 _seed_2))
  (bind _returnvalue_5 (Math|Random|RandomFloatinRangefromStream _returnvalue_3 _distance _seed_2))
  (bind _returnvalue_6 (+ _y _returnvalue_4))
  (bind _returnvalue_7 (+ _x _returnvalue_5))
  (bind _returnvalue_8 (Math|Vector|MakeVector _returnvalue_7 _returnvalue_6 _z))
  (for _index (range 0 (Variables|Default|GetTotalTrees))
    (bind _outhit (Collision|LineTraceByChannel _returnvalue_8 (- _returnvalue_8 (Math|Vector|MakeVector 0.0 0.0 (Variables|Default|GetZTraceDistance))) "TraceTypeQuery1" false 0 "ForDuration"))
    (if (Actor|ActorHasTag (.HitActor (Collision|BreakHitResult _outhit)) "landscape")
      (switch int (Math|Random|RandomIntegerinRangefromStream 0 2 _seed)
        (:0
          (Class|InstancedStaticMeshComponent|AddInstanceWorldSpace (Variables|Default|GetInstancedStaticMesh) (Math|Transform|MakeTransform (.Location (Collision|BreakHitResult _outhit)) (Math|Rotator|MakeRotator 0.0 0.0 (Math|Random|RandomFloatinRangefromStream 0.0 3.6e+02 _seed)) (Math|Conversions|ToVector(Float) (Math|Random|RandomFloatinRangefromStream 0.1 2.5 _seed)))))
        (:1
          (Class|InstancedStaticMeshComponent|AddInstanceWorldSpace (Variables|Default|GetInstancedStaticMesh1) (Math|Transform|MakeTransform (.Location (Collision|BreakHitResult _outhit)) (Math|Rotator|MakeRotator 0.0 0.0 (Math|Random|RandomFloatinRangefromStream 0.0 3.6e+02 _seed)) (Math|Conversions|ToVector(Float) (Math|Random|RandomFloatinRangefromStream 0.1 2.5 _seed)))))
        (:2
          (Class|InstancedStaticMeshComponent|AddInstanceWorldSpace (Variables|Default|GetInstancedStaticMesh2) (Math|Transform|MakeTransform (.Location (Collision|BreakHitResult _outhit)) (Math|Rotator|MakeRotator 0.0 0.0 (Math|Random|RandomFloatinRangefromStream 0.0 3.6e+02 _seed)) (Math|Conversions|ToVector(Float) (Math|Random|RandomFloatinRangefromStream 0.1 2.5 _seed)))))))))