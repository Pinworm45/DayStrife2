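; Player-driven boat pawn with VR-aware camera fades that can be exited at a dock or onto shore.
; Axis input adjusts clamped forward and turn speeds, applied by a looping timer and timeline with eased slowdown; hits halve forward speed.
; BuildMenu starts the ride once and attempts exit: spawning a TopDownCharacter at the first TargetPoint or on traced landscape-tagged ground, blending view, then possessing it after a delay.
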(event Custom|TickEvent
  ;[1 1 1] Tick / forward offset / rotation
  (bind _newtrack_0 (Timeline|Timeline_0 Play)
    (:Update
      (Transformation|AddActorLocalOffset (Math|Vector|MakeVector (* (Variables|Default|GetCurrentForwardSpeed) _newtrack_0) 0.0 0.0) true false)
      (Transformation|AddActorLocalRotation (Math|Rotator|MakeRotator 0.0 0.0 (* (Variables|Default|GetCurrentTurnSpeed) _newtrack_0)) false false)
      (if (and (== (Input|AxisValues|GetTurn) 0.0) (== (Input|AxisValues|GetTurnRate) 0.0))
        ;[1 1 1] Decrease Speeds based on Input
        (Variables|Default|SetCurrentTurnSpeed (Math|Interpolation|FInterpTo (Variables|Default|GetCurrentTurnSpeed) 0.0 (Utilities|Time|GetWorldDeltaSeconds) 1.0)))
      (if (== (Input|AxisValues|GetMoveForward) 0.0)
        (Variables|Default|SetCurrentForwardSpeed (Math|Interpolation|FInterpTo (Variables|Default|GetCurrentForwardSpeed) 0.0 (Utilities|Time|GetWorldDeltaSeconds) 0.4))))))

(event Collision|EventHit
  (params (MyComp :type Primitive%20Component%20Object%20Reference) (Other :type Actor%20Object%20Reference) (OtherComp :type Primitive%20Component%20Object%20Reference) (bSelfMoved :type Boolean) (HitLocation :type Vector :default "0, 0, 0") (HitNormal :type Vector :default "0, 0, 0") (NormalImpulse :type Vector :default "0, 0, 0") (Hit :type Hit%20Result%20Structure%20%28by%20ref%29))
  ;[1 1 1] Hit / slow speed
  (Variables|Default|SetCurrentForwardSpeed (/ (Variables|Default|GetCurrentForwardSpeed) 2.0)))

(event EventBeginPlay
  (bind _returnvalue (Game|GetPlayerController 0))
  ;[1 1 1] Begin Play, set input game only, camera fade
  (Input|SetInputModeGameOnly _returnvalue)
  (Variables|/Script/Engine.PlayerController|SetbShowMouseCursor _returnvalue false)
  (CameraFades|StartCameraFade :self (Game|GetPlayerCameraManager 0) :FromAlpha 1.5 :ToAlpha 1.5 :Duration 1.0 :bHoldWhenFinished true)
  (Utilities|Time|SetTimerbyEvent (delegate Custom|TickEvent) 0.01 true))

(event Input|ActionEvents|InputActionBuildMenu
  (params (Key :type Key%20Structure :default "AnyKey"))
  ;[1 1 1] Action / Exit Boat
  (:Pressed
    (Utilities|FlowControl|Sequence
      (:then_0
        ;[1 1 1] Start Game on F
        (Utilities|FlowControl|DoOnce false
          (:Completed
            (CameraFades|StartCameraFade :self (Game|GetPlayerCameraManager 0) :FromAlpha 1.5 :Duration 3.0)
            (Variables|Default|SetCurrentForwardSpeed -1e+01))))
      (:then_1
        (if (Variables|Default|GetAtDock)
          (CallFunction|ExittoDock)
          (else
            (CallFunction|ExittoShore)))))))

(event Input|AxisEvents|InputAxisMoveForward
  (params (AxisValue :type Float%20%28single-precision%29))
  ;[1 1 1] Forward Speed
  (if (!= AxisValue 0.0)
    (Variables|Default|SetCurrentForwardSpeed (Math|Float|Clamp(Float) (- (Variables|Default|GetCurrentForwardSpeed) (* AxisValue 0.02)) -12.0 12.0))))

(event Input|AxisEvents|InputAxisMoveRight
  (params (AxisValue :type Float%20%28single-precision%29))
  ;[1 1 1] Boat Turn
  (if (!= AxisValue 0.0)
    (Variables|Default|SetCurrentTurnSpeed (Math|Float|Clamp(Float) (+ (Variables|Default|GetCurrentTurnSpeed) (* AxisValue 0.005)) -1.0 1.0))))

(event Input|AxisEvents|InputAxisTurnRate
  (params (AxisValue :type Float%20%28single-precision%29))
  ;[1 1 1] Boat Turn
  (if (!= AxisValue 0.0)
    (Variables|Default|SetCurrentTurnSpeed (Math|Float|Clamp(Float) (+ (Variables|Default|GetCurrentTurnSpeed) (* AxisValue 0.005)) -1.0 1.0))))

(fn ConstructionScript)

(fn EnableController
  (bind _astop_down_controller (Utilities|Casting|CastToTopDownController (Game|GetPlayerController 0)))
  (Default|StartController _astop_down_controller))

(fn ExittoDock
  (bind _outactors (Actor|GetAllActorsOfClass "/Script/Engine.TargetPoint"))
  (bind _returnvalue (Game|SpawnActorfromClass "/Game/Blueprints/Pawns/TopDownCharacter.TopDownCharacter_C" (Math|Transform|MakeTransform (Transformation|GetActorLocation (Utilities|Array|Get(acopy) _outactors))) "Undefined" 0 0))
  (bind _output_get (Variables|Default|SetPawnToPossess _returnvalue))
  (Rendering|SetActorHiddenInGame _output_get true)
  (Game|Player|SetViewTargetwithBlend (Game|GetPlayerController 0) _output_get 1.0 "VTBlend_Linear" 1.0 false)
  (if (Class|HeadMountedDisplayFunctionLibrary|IsHeadMountedDisplayEnabled)
    (CameraFades|StartCameraFade :self (Game|GetPlayerCameraManager 0) :ToAlpha 1.0 :Duration 1.0 :bHoldWhenFinished true))
  (Utilities|Time|SetTimerbyFunctionName 0 "ExitBoat" 1.0))

(fn ExittoShore
  (bind _arrow (Variables|Default|GetArrow))
  (bind _returnvalue (Transformation|GetWorldLocation _arrow))
  (bind _outhit (Collision|LineTraceByChannel _returnvalue (- _returnvalue "0, 0,300.000000") "TraceTypeQuery1" false 0 "None"))
  (Utilities|IsValid (.HitActor (Collision|BreakHitResult _outhit))
    (:Is%20Valid
      (if (Actor|ActorHasTag (.HitActor (Collision|BreakHitResult _outhit)) "landscape")
        (bind _returnvalue_2 (Game|SpawnActorfromClass "/Game/Blueprints/Pawns/TopDownCharacter.TopDownCharacter_C" (Math|Transform|MakeTransform (+ (.Location (Collision|BreakHitResult _outhit)) "0, 0,100.000000")) "Undefined" 0 0))
        (bind _output_get (Variables|Default|SetPawnToPossess _returnvalue_2))
        (Rendering|SetActorHiddenInGame _output_get true)
        (Game|Player|SetViewTargetwithBlend (Game|GetPlayerController 0) _output_get 1.0 "VTBlend_Linear" 1.0 false)
        (if (Class|HeadMountedDisplayFunctionLibrary|IsHeadMountedDisplayEnabled)
          (CameraFades|StartCameraFade :self (Game|GetPlayerCameraManager 0) :ToAlpha 1.0 :Duration 1.0 :bHoldWhenFinished true))
        (Utilities|Time|SetTimerbyFunctionName 0 "ExitBoat" 1.0)))))

(fn ExitBoat
  (bind _returnvalue (Game|GetPlayerController 0))
  (bind _pawntopossess (Variables|Default|GetPawnToPossess))
  (Pawn|Possess _returnvalue _pawntopossess)
  (Input|SetInputModeGameOnly _returnvalue)
  (Variables|/Script/Engine.PlayerController|SetbShowMouseCursor _returnvalue false)
  (if (Class|HeadMountedDisplayFunctionLibrary|IsHeadMountedDisplayEnabled)
    (CameraFades|StartCameraFade :self (Game|GetPlayerCameraManager 0) :FromAlpha 2.0 :Duration 1.0))
  (Rendering|SetActorHiddenInGame _pawntopossess false))