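; Overseer pawn for a top-down building game, handling camera pan, zoom and ghost building placement.
; Movement axes offset the pawn locally unless the selection wheel is active.
; Mouse wheel and D-pad rotate the ghost building when one exists, otherwise they zoom the clamped spring arm.
; GhostBuild clears the TopDownController's selection, flags build mode and spawns the preview, which PlaceBuilding later tells to place itself.
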(event Input|AxisEvents|InputAxisMoveRight
  (params (AxisValue :type Float%20%28single-precision%29))
  ;[1 1 1] Movement
  (if (not (Variables|Default|GetSelectionWheelActive))
    (if (!= AxisValue 0.0)
      (Transformation|AddActorLocalOffset (Math|Vector|MakeVector 0.0 (* AxisValue 6e+01) 0.0) false false))))

(event Input|AxisEvents|InputAxisMoveForward
  (params (AxisValue :type Float%20%28single-precision%29))
  ;[1 1 1] Movement
  (if (not (Variables|Default|GetSelectionWheelActive))
    (if (!= AxisValue 0.0)
      (Transformation|AddActorLocalOffset (Math|Vector|MakeVector (* AxisValue 6e+01) 0.0 0.0) false false))))

(event Input|KeyboardEvents|1
  (params (Key :type Key%20Structure :default "AnyKey"))
  ;[1 1 1] Build House
  (:Pressed
    (CallFunction|GhostBuild "NewEnumerator0" "0, 0, 0")))

(event Input|GamepadEvents|GamepadDPadRight
  (params (Key :type Key%20Structure :default "AnyKey"))
  (bind _ghostbuilding (Variables|Default|GetGhostBuilding))
  (bind _springarm (Variables|Default|GetSpringArm))
  ;[1 1 1] Rotate Building / Zoom
  (:Pressed
    (if (Utilities|IsValid _ghostbuilding)
      (Transformation|AddActorLocalRotation _ghostbuilding "0,10.000000,0.000000" false false)
      (else
        (Variables|/Script/Engine.SpringArmComponent|SetTargetArmLength _springarm (Math|Float|Clamp(Float) (- (Variables|/Script/Engine.SpringArmComponent|GetTargetArmLength _springarm) 1.5e+02) -2.5e+03 2.5e+03))))))

(event Input|GamepadEvents|GamepadDPadLeft
  (params (Key :type Key%20Structure :default "AnyKey"))
  (bind _ghostbuilding (Variables|Default|GetGhostBuilding))
  (bind _springarm (Variables|Default|GetSpringArm))
  ;[1 1 1] Rotate Building / Zoom
  (:Pressed
    (if (Utilities|IsValid _ghostbuilding)
      (Transformation|AddActorLocalRotation _ghostbuilding "0,-10.000000,0.000000" false false)
      (else
        (Variables|/Script/Engine.SpringArmComponent|SetTargetArmLength _springarm (Math|Float|Clamp(Float) (+ (Variables|/Script/Engine.SpringArmComponent|GetTargetArmLength _springarm) 1.5e+02) -2.5e+03 2.5e+03))))))

(event Input|GamepadEvents|GamepadDPadUp
  (params (Key :type Key%20Structure :default "AnyKey"))
  (bind _ghostbuilding (Variables|Default|GetGhostBuilding))
  (bind _springarm (Variables|Default|GetSpringArm))
  ;[1 1 1] Rotate Building / Zoom
  (:Pressed
    (if (Utilities|IsValid _ghostbuilding)
      (Transformation|AddActorLocalRotation _ghostbuilding "0,10.000000,0.000000" false false)
      (else
        (Variables|/Script/Engine.SpringArmComponent|SetTargetArmLength _springarm (Math|Float|Clamp(Float) (- (Variables|/Script/Engine.SpringArmComponent|GetTargetArmLength _springarm) 1.5e+02) -2.5e+03 2.5e+03))))))

(event Input|GamepadEvents|GamepadDPadDown
  (params (Key :type Key%20Structure :default "AnyKey"))
  (bind _ghostbuilding (Variables|Default|GetGhostBuilding))
  (bind _springarm (Variables|Default|GetSpringArm))
  ;[1 1 1] Rotate Building / Zoom
  (:Pressed
    (if (Utilities|IsValid _ghostbuilding)
      (Transformation|AddActorLocalRotation _ghostbuilding "0,-10.000000,0.000000" false false)
      (else
        (Variables|/Script/Engine.SpringArmComponent|SetTargetArmLength _springarm (Math|Float|Clamp(Float) (+ (Variables|/Script/Engine.SpringArmComponent|GetTargetArmLength _springarm) 1.5e+02) -2.5e+03 2.5e+03))))))

(event Input|MouseEvents|MouseWheelUp
  (params (Key :type Key%20Structure :default "AnyKey"))
  (bind _ghostbuilding (Variables|Default|GetGhostBuilding))
  (bind _springarm (Variables|Default|GetSpringArm))
  ;[1 1 1] Rotate Building / Zoom
  (:Pressed
    (if (Utilities|IsValid _ghostbuilding)
      (Transformation|AddActorLocalRotation _ghostbuilding "0,10.000000,0.000000" false false)
      (else
        (Variables|/Script/Engine.SpringArmComponent|SetTargetArmLength _springarm (Math|Float|Clamp(Float) (- (Variables|/Script/Engine.SpringArmComponent|GetTargetArmLength _springarm) 1.5e+02) -2.5e+03 2.5e+03))))))

(event Input|MouseEvents|MouseWheelDown
  (params (Key :type Key%20Structure :default "AnyKey"))
  (bind _ghostbuilding (Variables|Default|GetGhostBuilding))
  (bind _springarm (Variables|Default|GetSpringArm))
  ;[1 1 1] Rotate Building / Zoom
  (:Pressed
    (if (Utilities|IsValid _ghostbuilding)
      (Transformation|AddActorLocalRotation _ghostbuilding "0,-10.000000,0.000000" false false)
      (else
        (Variables|/Script/Engine.SpringArmComponent|SetTargetArmLength _springarm (Math|Float|Clamp(Float) (+ (Variables|/Script/Engine.SpringArmComponent|GetTargetArmLength _springarm) 1.5e+02) -2.5e+03 2.5e+03))))))

(fn ConstructionScript)

(fn GhostBuild
  (params (enum :type BuildingsEnum%20Enum) (Rotation :type Rotator))
  (bind _astop_down_controller (Utilities|Casting|CastToTopDownController (Game|GetPlayerController 0)))
  (Class|Commandable|Deselect(Message) (Variables|/Game/Blueprints/Controllers/TopDownController.TopDownController_C|GetSelectedActors _astop_down_controller))
  (Utilities|Array|Clear (Variables|/Game/Blueprints/Controllers/TopDownController.TopDownController_C|GetSelectedActors _astop_down_controller))
  (Variables|/Game/Blueprints/Controllers/TopDownController.TopDownController_C|SetIsBuilding _astop_down_controller true)
  (bind _returnvalue (Game|SpawnActorfromClass "/Game/Blueprints/Buildings/BaseGhostBuilding.BaseGhostBuilding_C" (Math|Transform|MakeTransform "0, 0, 0" Rotation "2.000000,2.000000,2.000000") "Undefined" 0 enum 0))
  (Variables|Default|SetGhostBuilding _returnvalue))

(fn PlaceBuilding
  (Default|PlaceBuilding (Variables|Default|GetGhostBuilding)))