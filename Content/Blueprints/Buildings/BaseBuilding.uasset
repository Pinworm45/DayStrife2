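; BaseBuilding is a building actor Blueprint whose mesh can switch between visual states.
; On BeginPlay it caches the mesh's first material as the default.
; Custom events swap that material slot to a green vertex-color view material for highlighting, to a glass material, or back to the cached default.
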(event EventBeginPlay
  (Variables|Default|SetDefaultMat (Rendering|Material|GetMaterial (Variables|Default|GetBuildingMesh) 0)))

(event Collision|EventActorBeginOverlap
  (params (OtherActor :type Actor%20Object%20Reference)))

(event EventTick
  (params (DeltaSeconds :type Float%20%28single-precision%29)))

(event EventHighlightBuilding
  (Rendering|Material|SetMaterial (Variables|Default|GetBuildingMesh) 0 "/Engine/EngineDebugMaterials/VertexColorViewMode_GreenOnly.VertexColorViewMode_GreenOnly"))

(event EventGlassBuildings
  (Rendering|Material|SetMaterial (Variables|Default|GetBuildingMesh) 0 "/Game/Materials/Mat_Glass.Mat_Glass"))

(event EventRestoreBuildings
  (Rendering|Material|SetMaterial (Variables|Default|GetBuildingMesh) 0 (Variables|Default|GetDefaultMat)))

(fn ConstructionScript)