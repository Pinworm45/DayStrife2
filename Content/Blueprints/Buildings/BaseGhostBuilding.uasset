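; Placement preview actor for buildings, showing a glass-material mesh chosen by BuildingType.
; A looping timer snaps the mesh to the Pawn_Overseer cursor decal.
; Overlap events track blocking actors, turning the mesh red and clearing CanPlaceBuilding on the TopDownController until none remain.
; PlaceBuilding spawns the matching building class at the ghost's transform with a random seed, then destroys the ghost.
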(event OnComponentBeginOverlap(GhostBuildingMesh)
  (params (OverlappedComponent :type Primitive%20Component%20Object%20Reference) (OtherActor :type Actor%20Object%20Reference) (OtherComp :type Primitive%20Component%20Object%20Reference) (OtherBodyIndex :type Integer) (bFromSweep :type Boolean) (SweepResult :type Hit%20Result%20Structure%20%28by%20ref%29))
  ;[1 1 1] Overlapping
  (Rendering|Material|SetMaterial (Variables|Default|GetGhostBuildingMesh) 0 "/Game/Materials/Mat_red.Mat_red")
  (Utilities|Array|Add (Variables|Default|GetOverlappingActors) OtherActor)
  (bind _astop_down_controller (Utilities|Casting|CastToTopDownController (Game|GetPlayerController 0)))
  (Variables|/Game/Blueprints/Controllers/TopDownController.TopDownController_C|SetCanPlaceBuilding _astop_down_controller false))

(event OnComponentEndOverlap(GhostBuildingMesh)
  (params (OverlappedComponent :type Primitive%20Component%20Object%20Reference) (OtherActor :type Actor%20Object%20Reference) (OtherComp :type Primitive%20Component%20Object%20Reference) (OtherBodyIndex :type Integer))
  ;[1 1 1] Overlapping
  (Utilities|Array|RemoveItem (Variables|Default|GetOverlappingActors) OtherActor)
  (bind _astop_down_controller (Utilities|Casting|CastToTopDownController (Game|GetPlayerController 0)))
  (if (== (Utilities|Array|Length (Variables|Default|GetOverlappingActors)) 0)
    (Rendering|Material|SetMaterial (Variables|Default|GetGhostBuildingMesh) 0 "/Game/Materials/Mat_Glass.Mat_Glass")
    (Variables|/Game/Blueprints/Controllers/TopDownController.TopDownController_C|SetCanPlaceBuilding _astop_down_controller true)))

(event Custom|PutGhostUnderCursor
  (bind _aspawn_overseer (Utilities|Casting|CastToPawn_Overseer (Game|Player|GetPlayerPawn 0)))
  (Transformation|SetWorldLocation (Variables|Default|GetGhostBuildingMesh) (.Location (Math|Transform|BreakTransform (Transformation|GetWorldTransform (Variables|/Game/Blueprints/Pawns/Pawn_Overseer.Pawn_Overseer_C|GetDecal _aspawn_overseer)))) false false))

(event EventBeginPlay
  (bind _ghostbuildingmesh (Variables|Default|GetGhostBuildingMesh))
  (Utilities|Time|SetTimerbyEvent (delegate Custom|PutGhostUnderCursor) 0.01 true)
  (switch Utilities|FlowControl|Switch|SwitchonBuildingsEnum (Variables|Default|GetBuildingType)
    (:NewEnumerator0
      (Components|StaticMesh|SetStaticMesh _ghostbuildingmesh "/Game/TopDownCity/Houses/House1_01.House1_01"))
    (:NewEnumerator2
      (Components|StaticMesh|SetStaticMesh _ghostbuildingmesh "/Game/TopDownCity/Houses/House1_07.House1_07"))
    (:NewEnumerator3
      (Components|StaticMesh|SetStaticMesh _ghostbuildingmesh "/Game/TopDownCity/Houses/House1_03.House1_03"))
    (:NewEnumerator4
      (Components|StaticMesh|SetStaticMesh _ghostbuildingmesh "/Game/TopDownCity/Houses/House1_15.House1_15")))
  (Variables|Default|SetBuildingMaterial (Rendering|Material|GetMaterial (Variables|Default|GetGhostBuildingMesh) 0))
  (Rendering|Material|SetMaterial (Variables|Default|GetGhostBuildingMesh) 0 "/Game/Materials/Mat_Glass.Mat_Glass"))

(fn ConstructionScript)

(fn PlaceBuilding
  (bind _returnvalue (Math|Random|RandomIntegerinRange 0 50000))
  (bind _ghostbuildingmesh (Variables|Default|GetGhostBuildingMesh))
  (bind _returnvalue_2 (Math|Random|MakeRandomStream _returnvalue))
  (bind _returnvalue_3 (Transformation|GetWorldTransform _ghostbuildingmesh))
  (switch Utilities|FlowControl|Switch|SwitchonBuildingsEnum (Variables|Default|GetBuildingType)
    (:NewEnumerator0
      (Game|SpawnActorfromClass "/Game/Blueprints/Buildings/Building_House1.Building_House1_C" _returnvalue_3 "AlwaysSpawn" 0 _returnvalue_2 "NewEnumerator0"))
    (:NewEnumerator2
      (Game|SpawnActorfromClass "/Game/Blueprints/Buildings/Building_Warehouse.Building_Warehouse_C" _returnvalue_3 "AlwaysSpawn" 0 0 0 _returnvalue_2 "NewEnumerator2"))
    (:NewEnumerator3
      (Game|SpawnActorfromClass "/Game/Blueprints/Buildings/Building_Blacksmith.Building_Blacksmith_C" _returnvalue_3 "AlwaysSpawn" 0 _returnvalue_2 "NewEnumerator3"))
    (:NewEnumerator4
      (Game|SpawnActorfromClass "/Game/Blueprints/Buildings/Building_Tower.Building_Tower_C" _returnvalue_3 "AlwaysSpawn" 0 _returnvalue_2 "NewEnumerator4")))
  (Actor|DestroyActor))