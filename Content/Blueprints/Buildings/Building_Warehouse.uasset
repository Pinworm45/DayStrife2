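; Warehouse building where characters drop off the resources they carry.
; Overlapping the Entrance component makes an Old_TopDownChar or Pawn_TDC_Citizen add its resources to this warehouse and clears its HasTask flag.
; For citizens that are not possessed, it also sets the weight-limit Blackboard key to false.
; Construction only runs the parent script.
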(event OnComponentBeginOverlap(Entrance)
  (params (OverlappedComponent :type Primitive%20Component%20Object%20Reference) (OtherActor :type Actor%20Object%20Reference) (OtherComp :type Primitive%20Component%20Object%20Reference) (OtherBodyIndex :type Integer) (bFromSweep :type Boolean) (SweepResult :type Hit%20Result%20Structure%20%28by%20ref%29))
  (bind _self self)
  (bind _asold_top_down_char (Utilities|Casting|CastToOld_TopDownChar OtherActor)
    (:then
      (Default|AddResourcestoWarehouse _asold_top_down_char _self)
      (Variables|/Game/Blueprints/Pawns/Old_TopDownChar.Old_TopDownChar_C|SetHasTask _asold_top_down_char false))
    (:CastFailed
      (bind _aspawn_tdc_citizen (Utilities|Casting|CastToPawn_TDC_Citizen OtherActor))
      (Default|AddResourcestoWarehouse _aspawn_tdc_citizen _self)
      (Variables|/Game/Blueprints/Pawns/Pawn_TDC_Citizen.Pawn_TDC_Citizen_C|SetHasTask _aspawn_tdc_citizen false)
      (if (not (Variables|/Game/Blueprints/Pawns/Pawn_TDC_Citizen.Pawn_TDC_Citizen_C|GetPossessed _aspawn_tdc_citizen))
        (AI|Components|Blackboard|SetValueasBool (AI|GetBlackboard _aspawn_tdc_citizen) (Variables|Default|GetWeightLimitKey) false)))))

(event EventBeginPlay)

(event Collision|EventActorBeginOverlap
  (params (OtherActor :type Actor%20Object%20Reference)))

(event EventTick
  (params (DeltaSeconds :type Float%20%28single-precision%29)))

(fn ConstructionScript
  (|CallParentFunction))